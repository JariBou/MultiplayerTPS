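; Multiplayer game mode that spawns or respawns players as third-person characters at random Player Starts.
; SpawnPlayer destroys the controller's current pawn, spawns a BP_Character_TPS with collision adjustment and possesses it.
; Player Starts are cached on BeginPlay, and gathered on demand if the list is empty, since a PlayerController's BeginPlay can run first in builds.
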(event EventBeginPlay
  (Utilities|GatherPlayerStarts))

(event EventTick
  (params (DeltaSeconds :type Float%20%28single-precision%29)))

(fn ConstructionScript)

(fn FindRandomPlayerStart
  (bind _playerstarts (Variables|Default|GetPlayerStarts))
  (if (Utilities|Array|IsEmpty _playerstarts)
    ;[1 1 1] PC's BeginPlay Called first on build
    (Utilities|GatherPlayerStarts))
  (return (Transformation|GetActorTransform (.OutItem (Utilities|Array|Random _playerstarts)))))

(fn SpawnPlayer
  (params (PlayerController :type Player%20Controller%20Object%20Reference))
  (bind _returnvalue (Pawn|GetControlledPawn PlayerController))
  (bind _transform (CallFunction|FindRandomPlayerStart))
  (Utilities|IsValid _returnvalue
    (:Is%20Valid
      (Actor|DestroyActor _returnvalue))
    (:Is%20Not%20Valid
      _))
  (bind _returnvalue_2 (Game|SpawnActorfromClass "/Game/_project/BP/BP_Character_TPS.BP_Character_TPS_C" (Math|Transform|MakeTransform (.location _transform) (.rotation _transform) "1.000000,1.000000,1.000000") "AdjustIfPossibleButAlwaysSpawn" "MultiplyWithRoot" 0 0))
  (Pawn|Possess PlayerController _returnvalue_2))