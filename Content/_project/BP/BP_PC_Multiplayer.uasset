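; Multiplayer player controller that requests its pawn spawn on BeginPlay when locally controlled, and again after a short delay on player death.
; A server event has BP_GM_Multiplayer spawn the player for this controller.
; A multicast event then sets game-only input and hides the cursor, a fix for joining players being unable to control their character.
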(event Custom|MC_SpawnPlayer
  (params (PlayerController :type Player%20Controller%20Object%20Reference))
  ;[1 1 1] Fixes joining player not being able to control player
  (Input|SetInputModeGameOnly PlayerController true)
  (Variables|/Script/Engine.PlayerController|SetbShowMouseCursor PlayerController false))

(event Custom|ROS_SpawnPlayer
  (bind _self self)
  (Networking|SwitchHasAuthority
    (:Authority
      (bind _asbp_gm_multiplayer (Utilities|Casting|CastToBP_GM_Multiplayer (Game|GetGameMode)))
      (Default|SpawnPlayer _asbp_gm_multiplayer _self)
      (CallFunction|MCSpawnPlayer _self))))

(event Custom|PlayerDeath
  (Utilities|FlowControl|Delay 2.0)
  (CallFunction|ROSSpawnPlayer))

(event EventBeginPlay
  (Utilities|IsLocalPlayerControllerMacro
    (:True
      (CallFunction|ROSSpawnPlayer))))

(fn ConstructionScript)