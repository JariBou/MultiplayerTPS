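; BP_SniperRifle is a sniper rifle weapon Blueprint that adds a scope-style zoom while aiming.
; It implements the AimHook event to drive the owner's follow camera field of view from an alpha and an aiming flag.
; Aiming blends from the base FOV toward a fifth of it, while releasing blends from the current FOV back to base.
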(event EventBeginPlay
  (|CallParentFunction) ; This node is disabled and will not be called.\nDrag off pins to build functionality.
)

(event Collision|EventActorBeginOverlap
  (params (OtherActor :type Actor%20Object%20Reference))
  (|CallParentFunction OtherActor) ; This node is disabled and will not be called.\nDrag off pins to build functionality.
)

(event EventTick
  (params (DeltaSeconds :type Float%20%28single-precision%29))
  (|CallParentFunction DeltaSeconds) ; This node is disabled and will not be called.\nDrag off pins to build functionality.
)

(event EventAimHook
  (params (Alpha :type Float%20%28double-precision%29) (Aiming :type Boolean))
  (bind _selfowner (Variables|Default|GetSelfOwner))
  (bind _basecamerafov (Variables|/Game/_project/BP/BP_Character_TPS.BP_Character_TPS_C|GetBaseCameraFOV _selfowner))
  (Camera|SetFieldOfView (Variables|/Game/_project/BP/BP_Character_TPS.BP_Character_TPS_C|GetFollowCamera (Variables|Default|GetSelfOwner)) (Math|Float|SelectFloat (Math|Float|Lerp _basecamerafov (* _basecamerafov 0.2) Alpha) (Math|Float|Lerp (Variables|/Script/Engine.CameraComponent|GetFieldOfView (Variables|/Game/_project/BP/BP_Character_TPS.BP_Character_TPS_C|GetFollowCamera _selfowner)) _basecamerafov Alpha) Aiming)))

(fn ConstructionScript
  (|CallParentFunction))