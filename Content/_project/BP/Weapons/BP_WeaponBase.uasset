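; Base weapon Blueprint for networked hitscan shooting, fired from the owner's camera passed in through PassOwner.
; Fire calls a server event that line-traces, then multicasts the fire animation and surface-specific impact particles and sounds, skipped on dedicated servers.
; Body and head hits apply different damage by physical surface.
; A second trace behind those hits spawns randomly rolled blood splats scaled by distance.
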(event EventBeginPlay)

(event Collision|EventActorBeginOverlap
  (params (OtherActor :type Actor%20Object%20Reference)))

(event EventTick
  (params (DeltaSeconds :type Float%20%28single-precision%29)))

(event EventPassOwner
  (params (Owner :type Actor%20Object%20Reference) (OwnerCamera :type Camera%20Component%20Object%20Reference))
  (Variables|Default|SetSelfOwner Owner)
  (Variables|Default|SetOwner%20Camera OwnerCamera))

(event Custom|ROS_Fire
  (bind _owner_camera (Variables|Default|GetOwner%20Camera))
  (bind _returnvalue (Transformation|GetWorldLocation _owner_camera))
  (bind _returnvalue_2 (Math|Vector|GetForwardVector _owner_camera))
  ;[1 1 1] Shooting DOESN'T FUCKING WORK FOR SOME REASON   | Note from future me: works now... noob
  (Networking|SwitchHasAuthority
    (:Authority
      (bind (_outhit _returnvalue_3) (Collision|LineTraceByChannel _returnvalue (+ _returnvalue (* _returnvalue_2 1.5e+04)) "TraceTypeQuery3" false 0 "None"))
      (CallFunction|MCSpawnFX _returnvalue_3 (.Location (Collision|BreakHitResult _outhit)) (.Normal (Collision|BreakHitResult _outhit)) (.PhysMat (Collision|BreakHitResult _outhit)))
      (if _returnvalue_3
        (CallFunction|CallApplyDamage (.PhysMat (Collision|BreakHitResult _outhit)) (.HitActor (Collision|BreakHitResult _outhit)))
        (bind (_outhit_2 _returnvalue_4) (Collision|LineTraceByChannel (.Location (Collision|BreakHitResult _outhit)) (+ (.Location (Collision|BreakHitResult _outhit)) (* _returnvalue_2 1e+03)) "TraceTypeQuery4" false 0 "None" true "(R=0.000000,G=0.197003,B=1.000000,A=1.000000)" "(R=1.000000,G=0.727268,B=0.000000,A=1.000000)" 1.0))
        (if _returnvalue_4
          (switch Utilities|FlowControl|Switch|SwitchonEPhysicalSurface (Variables|/Script/PhysicsCore.PhysicalMaterial|GetSurfaceType (.PhysMat (Collision|BreakHitResult _outhit)))
            (:SurfaceType1
              _)
            (:SurfaceType4
              _))
          (Game|SpawnActorfromClass "/Game/Megascans/Decals/High_Velocity_Blood_Spatter_se1kfffp/BP_BloodSlat.BP_BloodSlat_C" (Math|Transform|MakeTransform (.Location (Collision|BreakHitResult _outhit_2)) (Math|Rotator|Delta(Rotator) (Class|KismetMathLibrary|NegateRotator (Math|Conversions|RotationFromXVector (.Normal (Collision|BreakHitResult _outhit_2)))) (Math|Rotator|MakeRotator (Math|Random|RandomFloatinRange -1.8e+02 1.8e+02) 0.0 0.0)) (Math|Conversions|ToVector(Float) (* (Math|Random|RandomFloatinRange 0.1 0.2) (* (Math|Vector|VectorLength (- (.ImpactPoint (Collision|BreakHitResult _outhit_2)) (.TraceStart (Collision|BreakHitResult _outhit_2)))) 0.02)))) "AlwaysSpawn" "MultiplyWithRoot" 0 0))))))

(event Custom|MC_SpawnFX
  (params (Hit :type Boolean) (HitLocation :type Vector) (HitNormal :type Vector) (PhysicalMaterial :type Physical%20Material%20Object%20Reference))
  ;[1 1 1] Shooting DOESN'T FUCKING WORK FOR SOME REASON   | Note from future me: works now... noob
  (if (not (Networking|IsDedicatedServer))
    (bind _mesh (CallFunction|GetSkeletalMeshComponent))
    (Components|Animation|PlayAnimation _mesh "/Game/MilitaryWeapDark/Weapons/Anims/Fire_Rifle_W.Fire_Rifle_W" false)
    (if Hit
      (switch Utilities|FlowControl|Switch|SwitchonEPhysicalSurface (Variables|/Script/PhysicsCore.PhysicalMaterial|GetSurfaceType PhysicalMaterial)
        (:SurfaceType1
          (|SpawnParticles HitLocation (Math|Rotator|Delta(Rotator) (Math|Conversions|RotationFromXVector HitNormal) "90.000000,0.000000,0.000000") :!label _label))
        (:SurfaceType2
          (goto _label Asphalt))
        (:SurfaceType3
          (goto _label Metal))
        (:SurfaceType4
          (goto _label Head))))))

(event EventFire
  ;[1 1 1] Shooting DOESN'T FUCKING WORK FOR SOME REASON   | Note from future me: works now... noob
  (CallFunction|ROSFire))

(fn ConstructionScript)

(fn CallApplyDamage
  (params (PhysicalMaterial :type Physical%20Material%20Object%20Reference) (DamagedActor :type Actor%20Object%20Reference))
  (bind _selfowner (Variables|Default|GetSelfOwner))
  (switch Utilities|FlowControl|Switch|SwitchonEPhysicalSurface (Variables|/Script/PhysicsCore.PhysicalMaterial|GetSurfaceType PhysicalMaterial)
    (:SurfaceType1
      (Game|Damage|ApplyDamage DamagedActor 25.0 0 _selfowner "/Script/Engine.DamageType"))
    (:SurfaceType4
      (Game|Damage|ApplyDamage DamagedActor 1.5e+02 0 _selfowner "/Script/Engine.DamageType"))))

(fn SpawnEmitterandSound
  (params (EmitterTemplate :type Particle%20System%20Object%20Reference) (Location :type Vector) (Rotation :type Rotator) (Scale :type Vector) (Sound :type Sound%20Base%20Object%20Reference))
  (Effects|SpawnEmitteratLocation EmitterTemplate Location Rotation Scale)
  (Audio|PlaySoundatLocation Sound Location "0, 0, 0" 1.0 1.0 0.0 0 0 0 0))

(fn GetSkeletalMeshComponent
  (return (Variables|Default|GetWeaponMesh)))

(fn GetWeaponFamily
  (return (Variables|Default|GetWeaponFamily)))